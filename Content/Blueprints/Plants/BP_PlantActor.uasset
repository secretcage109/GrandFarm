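; Plant actor that withers away when a first-stage tomato is left on dry dirt.
; An actor overlap starts a roughly four-minute Delay, then checks whether the mesh is still TomatoLv1.
; If so, it scans dirt actors overlapping its Box and destroys itself at the first one lacking the wet ground material.
; The DoOnce resets as soon as the Delay starts, so later overlaps can start another check once it finishes.
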(event `Destory actor`
  (`KismetSystemLibrary.Delay` 0.0)
  (`self.K2_DestroyActor`))

(event `self.ReceiveActorBeginOverlap`
  (params (OtherActor :type "Actor Object Reference"))
  (`/Engine/EditorBlueprintResources/StandardMacros.DoOnce` false :!label _label
    (:`Completed`
      (`|ExecutionSequence`
        (:`then_0`
          (`KismetSystemLibrary.Delay` 245.02)
          (if (== (`StaticMeshComponent.StaticMesh` (`self.MeshComponent`)) "/Game/Item/Consumable/Tomato/TomatoLv1.TomatoLv1")
            (for _array_element (`PrimitiveComponent.GetOverlappingActors` (`self.Box`) "/Game/MapArts/Blueprints/Props/BP_CollisionGroundDirt.BP_CollisionGroundDirt_C")
              (bind _asbp_collision_ground_dirt (cast `/Game/MapArts/Blueprints/Props/BP_CollisionGroundDirt` _array_element)
                (:`then`
                  (if (not (== (`PrimitiveComponent.GetMaterial` (`/Game/MapArts/Blueprints/Props/BP_CollisionGroundDirt.GroundDirt` _asbp_collision_ground_dirt) 0) "/Game/MapArts/Blueprints/MapArtMaterial/Mat_WetG.Mat_WetG"))
                    (`self.Destory actor`)
                    (break)))
                (:`CastFailed`
                  (`KismetSystemLibrary.PrintString` "캐스트 실패"))))))
        (:`then_1`
          (goto _label :!via `Reset`))))))

(event `self.ReceiveBeginPlay`)

(fn `UserConstructionScript`)