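; BP_Cloud is a drifting cloud actor whose movement scales with the GameSpeed of BP_GameTimeManager.
; Tick moves it along MovementDirection, wrapping past the X boundary to before the minimum with random Y and Z offsets.
; The construction script randomizes mesh scale and altitude and creates a dynamic material.
; It also rolls a random opacity, but DynamicMaterial is set to None before that value is applied.
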(event `self.ReceiveBeginPlay`
  (bind _returnvalue (`GameplayStatics.GetActorOfClass` "/Game/Blueprints/BP_GameTimeManager.BP_GameTimeManager_C"))
  (set `self.GameTimeManager` _returnvalue)
  (set `self.CurrentSpeed` (`self.BaseSpeed`)))

(event `self.ReceiveTick`
  (params (DeltaSeconds :type "Float (single-precision)"))
  (if (`KismetSystemLibrary.IsValid` (`self.GameTimeManager`))
    ;[1 1 1] 경계선
    (`self.K2_SetActorLocation` (+ (`self.K2_GetActorLocation`) (* (`self.MovementDirection`) (* (`self.CurrentSpeed`) (* (/ (`/Game/Blueprints/BP_GameTimeManager.GameSpeed` (`self.GameTimeManager`)) 60.0) DeltaSeconds)))))
    (if (>= (.x (`self.K2_GetActorLocation`)) (`self.MaxBoundary`))
      (`self.K2_SetActorLocation` (`KismetMathLibrary.MakeVector` (- (`self.MinBoundary`) 500.0) (+ (`KismetMathLibrary.RandomFloatInRange` -500.0 500.0) (.y (`self.K2_GetActorLocation`))) (+ (`KismetMathLibrary.RandomFloatInRange` -200.0 200.0) (.z (`self.K2_GetActorLocation`))))))))

(fn `UserConstructionScript`
  (bind _returnvalue (`KismetMathLibrary.RandomFloatInRange` 0.8 2.5))
  (`SceneComponent.SetRelativeScale3D` (`self.CloudMesh`) (`KismetMathLibrary.MakeVector` _returnvalue _returnvalue _returnvalue))
  (`self.K2_SetActorLocation` (`KismetMathLibrary.MakeVector` (.x (`self.K2_GetActorLocation`)) (.y (`self.K2_GetActorLocation`)) (`KismetMathLibrary.RandomFloatInRange` 1000.0 2000.0)))
  (`PrimitiveComponent.CreateDynamicMaterialInstance` (`self.CloudMesh`) 0 null "None")
  (set `self.DynamicMaterial` null)
  (bind _output_get (set `self.CloudOpacity` (`KismetMathLibrary.RandomFloatInRange` 0.4 0.8)))
  (`MaterialInstanceDynamic.SetScalarParameterValue` (`self.DynamicMaterial`) "Opacity" _output_get))