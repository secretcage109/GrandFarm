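; BP_MyPlayerController is a player controller that lets the player place plants in the world with a left click.
; BeginPlay shows the mouse cursor, enables input and turns off click events.
; Each left press traces the Visibility channel under the cursor and spawns BP_PlantActor there, snapping X and Y to a 100-unit grid and keeping the hit Z.
; The hit result is not validated, and DrawPlant is an empty stub.
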(event `self.ReceiveBeginPlay`
  (set `self.bShowMouseCursor` true)
  (`self.EnableInput` (`GameplayStatics.GetPlayerController` 0))
  (set `self.bEnableClickEvents` false))

(event `Key|LeftMouseButton`
  (params (Key :type "Key Structure"))
  (bind (_bblockinghit _binitialoverlap _time _distance _location) (`GameplayStatics.BreakHitResult` (`self.GetHitResultUnderCursorByChannel` "TraceTypeQuery1")))
  (:`Pressed`
    (`|SpawnActorFromClass` "/Game/Blueprints/Plants/BP_PlantActor.BP_PlantActor_C" (`KismetMathLibrary.MakeTransform` (`KismetMathLibrary.MakeVector` (`KismetMathLibrary.Conv_IntToDouble` (* (`KismetMathLibrary.Round` (/ (.x _location) 100.0)) 100)) (`KismetMathLibrary.Conv_IntToDouble` (* (`KismetMathLibrary.Round` (/ (.y _location) 100.0)) 100)) (.z _location))) "Undefined" "MultiplyWithRoot" null null)))

(fn `Draw Plant`)

(fn `UserConstructionScript`)