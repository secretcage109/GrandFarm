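; Game time manager that runs the day clock, sun movement and day rollover, and creates the time display widget.
; Tick advances the hour scaled by GameSpeed, then maps it onto the pitch of the first DirectionalLight found.
; At DayEndHour it resets to morning, increments the day and sets BP_WeatherManager's weather, forcing rain on day two.
; The CallOnDayChanged call is unconnected and never runs.
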(event `self.ReceiveBeginPlay`
  (`|ExecutionSequence`
    (:`then_0`
      (bind _outactors (`GameplayStatics.GetAllActorsOfClass` "/Script/Engine.DirectionalLight"))
      (set `self.SunLight` (`|GetArrayItem` _outactors)))
    (:`then_1`
      (bind _outactors_2 (`GameplayStatics.GetAllActorsOfClass` "/Game/Blueprints/BP_WeatherManager.BP_WeatherManager_C"))
      (set `self.WeatherManager` (`|GetArrayItem` _outactors_2)))
    (:`then_2`
      (bind _returnvalue (`|CreateWidget` "/Game/Blueprints/WBP_TimeDisplay.WBP_TimeDisplay_C"))
      (`UserWidget.AddToViewport` _returnvalue 0))))

(event `self.ReceiveTick`
  (params (DeltaSeconds :type "Float (single-precision)"))
  ;[1 1 1] 시간 증가 계산
  (set `self.CurrentHour` (+ (`self.CurrentHour`) (/ (* DeltaSeconds 16.0) (`self.GameSpeed`))))
  (`self.UpdateSun`)
  (`self.CheckDayEnd`))

(event `UpdateSun`
  ;[1 1 1] 태양 회전
  (`self.K2_SetActorRotation` (`self.SunLight`) (`KismetMathLibrary.MakeRotator` 0.0 (* (`KismetMathLibrary.NormalizeToRange` (`self.CurrentHour`) 6.0 21.0) -180.0)) false))

(event `CheckDayEnd`
  ;[1 1 1] 하루 종료
  (if (>= (`self.CurrentHour`) (`self.DayEndHour`))
    (set `self.CurrentHour` 6.0)
    (set `self.CurrentDay` (+ (`self.CurrentDay`) 1))
    ;[1 1 1] 강제 2일차 비
    (if (== (`self.CurrentDay`) 2)
      (`/Game/Blueprints/BP_WeatherManager.ChangeWeather` (`self.WeatherManager`) 1)
      (else
        (`/Game/Blueprints/BP_WeatherManager.ChangeWeather` (`self.WeatherManager`) 0)))))

(fn `UserConstructionScript`)