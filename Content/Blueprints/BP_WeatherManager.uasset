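; Weather manager actor that picks clear or overcast weather whenever the game day changes.
; On BeginPlay it finds the level's directional light, height fog and BP_GameTimeManager, then binds to the day-changed event.
; Each day of a seven-day cycle rolls its own chance of bad weather, with one day always bad.
; ChangeWeather switches sun intensity and color, fog density, and a Niagara effect between the two presets.
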(event `self.ReceiveBeginPlay`
  (`|ExecutionSequence`
    (:`then_0`
      (bind _outactors (`GameplayStatics.GetAllActorsOfClass` "/Script/Engine.DirectionalLight"))
      (set `self.SunLight` (`|GetArrayItem` _outactors)))
    (:`then_1`
      (bind _outactors_2 (`GameplayStatics.GetAllActorsOfClass` "/Script/Engine.ExponentialHeightFog"))
      (set `self.Fog` (`|GetArrayItem` _outactors_2)))
    (:`then_2`
      (bind _outactors_3 (`GameplayStatics.GetAllActorsOfClass` "/Game/Blueprints/BP_GameTimeManager.BP_GameTimeManager_C"))
      (set `self.GameTimeManager` (`|GetArrayItem` _outactors_3))
      (add `/Game/Blueprints/BP_GameTimeManager.OnDayChanged` (`self.GameTimeManager`) (delegate `HandleDayChanged`)))))

(event `HandleDayChanged`
  (switch `int` (mod (`/Game/Blueprints/BP_GameTimeManager.CurrentDay` (`self.GameTimeManager`)) 7)
    (:`0`
      (if (< (`KismetMathLibrary.RandomFloatInRange` 0.0 1.0) 0.2)
        (`self.ChangeWeather` 1)
        (else
          (`self.ChangeWeather` 0))))
    (:`1`
      (`self.ChangeWeather` 1))
    (:`2`
      (if (< (`KismetMathLibrary.RandomFloatInRange` 0.0 1.0) 0.3)
        (`self.ChangeWeather` 1)
        (else
          (`self.ChangeWeather` 0))))
    (:`3`
      (if (< (`KismetMathLibrary.RandomFloatInRange` 0.0 1.0) 0.25)
        (`self.ChangeWeather` 1)
        (else
          (`self.ChangeWeather` 0))))
    (:`4`
      (if (< (`KismetMathLibrary.RandomFloatInRange` 0.0 1.0) 0.35)
        (`self.ChangeWeather` 1)
        (else
          (`self.ChangeWeather` 0))))
    (:`5`
      (if (< (`KismetMathLibrary.RandomFloatInRange` 0.0 1.0) 0.15)
        (`self.ChangeWeather` 1)
        (else
          (`self.ChangeWeather` 0))))
    (:`6`
      (if (< (`KismetMathLibrary.RandomFloatInRange` 0.0 1.0) 0.1)
        (`self.ChangeWeather` 1)
        (else
          (`self.ChangeWeather` 0))))))

(fn `ChangeWeather`
  (params (WeatherType :type Integer))
  (switch `int` WeatherType
    (:`0`
      (`LightComponent.SetIntensity` (`Light.LightComponent` (`self.SunLight`)) 8.0)
      (`LightComponent.SetLightColor` (`Light.LightComponent` (`self.SunLight`)) (struct :`R` 1.0 :`G` 0.9 :`B` 0.7 :`A` 1.0) true)
      (`ExponentialHeightFogComponent.SetFogDensity` (`ExponentialHeightFog.Component` (`self.Fog`)) 0.02)
      (`ActorComponent.Deactivate` (`self.Niagara`)))
    (:`1`
      (`LightComponent.SetIntensity` (`Light.LightComponent` (`self.SunLight`)) 2.0)
      (`LightComponent.SetLightColor` (`Light.LightComponent` (`self.SunLight`)) (struct :`R` 0.4 :`G` 0.4 :`B` 0.5 :`A` 1.0) true)
      (`ExponentialHeightFogComponent.SetFogDensity` (`ExponentialHeightFog.Component` (`self.Fog`)) 0.1)
      (`ActorComponent.Activate` (`self.Niagara`) false))))

(fn `UserConstructionScript`)