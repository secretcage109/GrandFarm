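; BP_WateringPickup is the world pickup for the Watering tool, which removes itself if the loaded inventory already contains that item.
; On BeginPlay it calls RegisterWatering on BP_GameInstance, then scans that instance's LoadedInventory and destroys the actor on a matching item name.
; The graph holds no pickup interaction logic, only this startup check and some unconnected debug prints.
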(event `self.ReceiveBeginPlay`
  (`parent.ReceiveBeginPlay`)
  (bind _asbp_game_instance (cast `/Game/Blueprints/BP_GameInstance` (`GameplayStatics.GetGameInstance`))
    (:`then`
      (`/Game/Blueprints/BP_GameInstance.RegisterWatering` _asbp_game_instance)
      (bind _asbp_game_instance_2 (cast `/Game/Blueprints/BP_GameInstance` (`GameplayStatics.GetGameInstance`)))
      (for _array_element (`/Game/Blueprints/BP_GameInstance.LoadedInventory` _asbp_game_instance_2)
        (if (== (`.ItemName_4_E272051245B9E4736895D5966FD47843` (break `/Game/Inventory/Inventory/S_Slot` _array_element)) "Watering")
          (`self.K2_DestroyActor`))))
    (:`CastFailed`
      (`KismetSystemLibrary.PrintString` "cast Failed"))))

(fn `UserConstructionScript`
  (`parent.UserConstructionScript`))