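; BP_Item is a world item that shows a widget and registers itself with the player when something overlaps its sphere.
; On BeginPlay it caches the player character as BP_Player2.
; Sphere begin overlap shows the widget and sets the player's Item reference to itself; end overlap hides it and clears the reference.
; The overlap handlers do not check which actor triggered them.
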(event `self.ReceiveBeginPlay`
  (bind _asbp_player_2 (cast `/Game/Player/BP_Player2` (`GameplayStatics.GetPlayerCharacter` 0)))
  (set `self.PlayerCharacter` _asbp_player_2))

(event `self.Sphere.OnComponentBeginOverlap`
  (params (OverlappedComponent :type "PrimitiveComponent Object Reference") (OtherActor :type "Actor Object Reference") (OtherComp :type "PrimitiveComponent Object Reference") (OtherBodyIndex :type Integer) (bFromSweep :type Boolean) (SweepResult :type "HitResult Structure (by ref)"))
  (`SceneComponent.SetVisibility` (`self.Widget`) true false)
  (bind _output_get (set `/Game/Player/BP_Player2.Item` self (`self.PlayerCharacter`))))

(event `self.Sphere.OnComponentEndOverlap`
  (params (OverlappedComponent :type "PrimitiveComponent Object Reference") (OtherActor :type "Actor Object Reference") (OtherComp :type "PrimitiveComponent Object Reference") (OtherBodyIndex :type Integer))
  (`SceneComponent.SetVisibility` (`self.Widget`) false false)
  (set `/Game/Player/BP_Player2.Item` null (`self.PlayerCharacter`)))

(fn `UserConstructionScript`)